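; Treasure chest actor that glitters and lights up while something is nearby.
; It starts dark, with the Glitter effect's asset cleared and four Illumination lights at zero intensity.
; Sphere begin overlap assigns the ChestGlitter asset and raises the lights to the Intensity variable, and end overlap reverts both.
; Overlaps are not filtered by actor or counted, so any end overlap switches everything off.
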(event OnComponentBeginOverlap(Sphere)
  (params (OverlappedComponent :type Primitive%20Component%20Object%20Reference) (OtherActor :type Actor%20Object%20Reference) (OtherComp :type Primitive%20Component%20Object%20Reference) (OtherBodyIndex :type Integer) (bFromSweep :type Boolean) (SweepResult :type Hit%20Result%20Structure%20%28by%20ref%29))
  (Class|NiagaraComponent|SetAsset (Variables|Default|GetGlitter) "/Game/Fab/Lowpoly_Treasure_Chest/ChestGlitter.ChestGlitter" true)
  (Rendering|Components|Light|SetIntensity (Variables|Default|GetIllumination) (Variables|Default|GetIntensity))
  (Rendering|Components|Light|SetIntensity (Variables|Default|GetIllumination2) (Variables|Default|GetIntensity))
  (Rendering|Components|Light|SetIntensity (Variables|Default|GetIllumination3) (Variables|Default|GetIntensity))
  (Rendering|Components|Light|SetIntensity (Variables|Default|GetIllumination4) (Variables|Default|GetIntensity)))

(event OnComponentEndOverlap(Sphere)
  (params (OverlappedComponent :type Primitive%20Component%20Object%20Reference) (OtherActor :type Actor%20Object%20Reference) (OtherComp :type Primitive%20Component%20Object%20Reference) (OtherBodyIndex :type Integer))
  (Class|NiagaraComponent|SetAsset (Variables|Default|GetGlitter) 0 true)
  (Rendering|Components|Light|SetIntensity (Variables|Default|GetIllumination) 0.0)
  (Rendering|Components|Light|SetIntensity (Variables|Default|GetIllumination2) 0.0)
  (Rendering|Components|Light|SetIntensity (Variables|Default|GetIllumination3) 0.0)
  (Rendering|Components|Light|SetIntensity (Variables|Default|GetIllumination4) 0.0))

(event EventBeginPlay
  (Class|NiagaraComponent|SetAsset (Variables|Default|GetGlitter) 0 true)
  (Rendering|Components|Light|SetIntensity (Variables|Default|GetIllumination) 0.0)
  (Rendering|Components|Light|SetIntensity (Variables|Default|GetIllumination2) 0.0)
  (Rendering|Components|Light|SetIntensity (Variables|Default|GetIllumination3) 0.0)
  (Rendering|Components|Light|SetIntensity (Variables|Default|GetIllumination4) 0.0))

(event Collision|EventActorBeginOverlap
  (params (OtherActor :type Actor%20Object%20Reference)))

(event EventTick
  (params (DeltaSeconds :type Float%20%28single-precision%29)))

(fn ConstructionScript)