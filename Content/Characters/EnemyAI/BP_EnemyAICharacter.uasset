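; Enemy AI character that detects the player by sight and sound and takes projectile damage.
; While the player is seen, line traces from the head to player body parts set how fast detection rises; otherwise it changes by DecreaseRate.
; Heard noises set blackboard keys, with HeardSound updated each tick by proximity to the location.
; Body hits deal half damage, head hits full, driving blood effects, health bar and destruction.
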(event OnSeePawn(PawnSensing)
  (params (Pawn :type Pawn%20Object%20Reference))
  (Variables|Default|SetSeesPlayer (== Pawn (Variables|Default|GetPlayerPawn)))
  (Variables|Default|SetLastSeenTime (Utilities|Time|GetGameTimeinSeconds)))

(event OnHearNoise(PawnSensing)
  (params (Instigator :type Pawn%20Object%20Reference) (Location :type Vector%20%28by%20ref%29 :default "0, 0, 0") (Volume :type Float%20%28single-precision%29))
  (bind _returnvalue (AI|GetBlackboard 0))
  (bind _output_get (Variables|Default|SetLastHeardLocation Location))
  (AI|Components|Blackboard|SetValueasVector _returnvalue (Utilities|Name|MakeLiteralName "SoundLocation") _output_get)
  (AI|Components|Blackboard|SetValueasBool _returnvalue (Utilities|Name|MakeLiteralName "HeardSound") true))

(event OnComponentHit(BodyCollisionCapsule)
  (params (HitComponent :type Primitive%20Component%20Object%20Reference) (OtherActor :type Actor%20Object%20Reference) (OtherComp :type Primitive%20Component%20Object%20Reference) (NormalImpulse :type Vector :default "0, 0, 0") (Hit :type Hit%20Result%20Structure%20%28by%20ref%29))
  (bind _asbp_projectile (Utilities|Casting|CastToBP_Projectile OtherActor))
  (CallFunction|HitbyProjectile (* (Variables|/Game/Inventory/BP_Projectile.BP_Projectile_C|GetDamage _asbp_projectile) 0.5))
  (CallFunction|SpawnBloodParticles (.impactpoint Hit) (.normal Hit)))

(event OnComponentHit(HeadCollisionSphere)
  (params (HitComponent :type Primitive%20Component%20Object%20Reference) (OtherActor :type Actor%20Object%20Reference) (OtherComp :type Primitive%20Component%20Object%20Reference) (NormalImpulse :type Vector :default "0, 0, 0") (Hit :type Hit%20Result%20Structure%20%28by%20ref%29))
  (bind _asbp_projectile (Utilities|Casting|CastToBP_Projectile OtherActor))
  (CallFunction|HitbyProjectile (* (Variables|/Game/Inventory/BP_Projectile.BP_Projectile_C|GetDamage _asbp_projectile) 1.0))
  (CallFunction|SpawnBloodParticles (.location Hit) (.normal Hit)))

(event EventBeginPlay
  (bind _asbp_player_pawn (Utilities|Casting|CastToBP_PlayerPawn (Game|Player|GetPlayerPawn 0)))
  (Variables|Default|SetPlayerPawn _asbp_player_pawn))

(event Collision|EventActorBeginOverlap
  (params (OtherActor :type Actor%20Object%20Reference)))

(event EventTick
  (params (DeltaSeconds :type Float%20%28single-precision%29))
  (Utilities|FlowControl|Sequence
    (:then_0
      (CallFunction|CheckifAlive))
    (:then_1
      (CallFunction|CheckifLostSightOfPlayer))
    (:then_2
      (CallFunction|UpdateDetectionLevel DeltaSeconds))
    (:then_3
      (CallFunction|CheckifReachedSoundLocation))))

(fn ConstructionScript)

(fn ComputeEnemyVisibilityRatio
  (bind _values (Utilities|Map|Values (Variables|/Game/Characters/Player/BP_PlayerPawn.BP_PlayerPawn_C|GetBodyPartsLocation (Variables|Default|GetPlayerPawn))))
  (for _array_element _values
    (bind _isvisible (CallFunction|IsBodypartVisible _array_element))
    (if _isvisible
      (bind _result (Math|Float|IncrementFloat (LocalVariables|GetVisiblePartsCount))
        (:%20%20
          (LocalVariables|SetVisiblePartsCount _result)))))
  (return (/ (LocalVariables|GetVisiblePartsCount) (Utilities|Array|Length _values))))

(fn HitbyProjectile
  (params (Damage :type Float%20%28double-precision%29))
  (Variables|Default|SetHealth (- (Variables|Default|GetHealth) Damage))
  (CallFunction|UpdateHealthBar))

(fn UpdateHealthBar
  (bind _ashealth_bar (Utilities|Casting|CastToHealthBar (UserInterface|GetWidget (Variables|Default|GetHealthBarWidget))))
  (Variables|/Game/Characters/EnemyAI/HealthBar.HealthBar_C|SetHealth _ashealth_bar (Variables|Default|GetHealth)))

(fn CheckifAlive
  (if (<= (Variables|Default|GetHealth) 0.0)
    (Pawn|UnPossess (Pawn|GetController))
    (Actor|DestroyActor)))

(fn CheckifLostSightOfPlayer
  (if (< (Variables|Default|GetLoseSightDelay) (- (Utilities|Time|GetGameTimeinSeconds) (Variables|Default|GetLastSeenTime)))
    (Variables|Default|SetSeesPlayer false)))

(fn UpdateDetectionLevel
  (params (DeltaSeconds :type Float%20%28double-precision%29))
  (Variables|Default|SetDetectionLevel (Math|Float|Clamp(Float) (+ (* DeltaSeconds (select (Variables|Default|GetSeesPlayer) (CallFunction|ComputeEnemyVisibilityRatio) (Variables|Default|GetDecreaseRate))) (Variables|Default|GetDetectionLevel))))
  (CallFunction|UpdateDetectionBar))

(fn IsBodypartVisible
  (params (TargetBodypartLocation :type Vector))
  (bind _headcollisionsphere (Variables|Default|GetHeadCollisionSphere))
  (if (Utilities|IsValid _headcollisionsphere)
    (bind _outhit (Collision|LineTraceByChannel (Transformation|GetSocketLocation _headcollisionsphere "None") TargetBodypartLocation "TraceTypeQuery1" false 0 "None"))
    (return (== (.hitactor _outhit) (Variables|Default|GetPlayerPawn)))))

(fn CheckifReachedSoundLocation
  (bind _asenemy_aicontroler (Utilities|Casting|CastToEnemyAIControler (Pawn|GetController)))
  (AI|Components|Blackboard|SetValueasBool (AI|GetBlackboard 0) (Utilities|Name|MakeLiteralName "HeardSound") (not (Default|IsNearLocation _asenemy_aicontroler (Variables|Default|GetLastHeardLocation)))))

(fn SpawnBloodParticles
  (params (HitImpactPoint :type Vector) (HitNormal :type Vector))
  (Niagara|SpawnSystematLocation "/Game/Characters/NS_BloodSplash.NS_BloodSplash" HitImpactPoint (Math|Rotator|MakeRotfromZ (* HitNormal -1.0))))

(fn UpdateDetectionBar
  (bind _asdetection_bar (Utilities|Casting|CastToDetectionBar (UserInterface|GetWidget (Variables|Default|GetDetectionBarWidget))))
  (Variables|/Game/Characters/EnemyAI/DetectionBar.DetectionBar_C|SetDetection _asdetection_bar (* (Variables|Default|GetDetectionLevel) 1e+02)))