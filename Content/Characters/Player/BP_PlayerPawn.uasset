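; Player character pawn that manages health, sprint and jump stamina, item pickups, quest completion and win/death level loading.
; Each Tick caches body-part socket locations, emits speed-scaled noise through PawnNoiseEmitter, updates stamina and opens the death level at zero health.
; A per-frame camera trace toggles interact prompts on the targeted rock or knife.
; Pickup functions update the HUD hotbar and destroy the targeted item.
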(event Custom|Update%20quest
  (params (QuestID :type Integer))
  (bind _questsarray (Variables|Default|GetQuestsArray))
  (bind _output (Utilities|Array|Get(acopy) _questsarray QuestID))
  (bind (_questid _title _objectivetext) (Utilities|Struct|BreakQuestStructure _output))
  (Utilities|Array|SetArrayElem _questsarray QuestID (Utilities|Struct|MakeQuestStructure _questid _title _objectivetext true)))

(event Collision|EventActorBeginOverlap
  (params (OtherActor :type Actor%20Object%20Reference)))

(event EventTick
  (params (DeltaSeconds :type Float%20%28single-precision%29))
  (Utilities|FlowControl|Sequence
    (:then_0
      (CallFunction|ComputeBodyPartsLocation))
    (:then_1
      (CallFunction|MakeSound))
    (:then_2
      (bind (_startpoint _endpoint) (CallFunction|CalculatePickUpRange))
      (bind _outhit (Collision|LineTraceByChannel _startpoint _endpoint "TraceTypeQuery3" false 0 "None"))
      (CallFunction|TrySetCurrentRockRef (.hitactor _outhit)))
    (:then_3
      (CallFunction|HandleStamina DeltaSeconds))
    (:then_4
      (bind _alive (CallFunction|IsAlive))
      (CallFunction|StopGame _alive))))

(event EventBeginPlay)

(fn ConstructionScript
  (Variables|/Script/Engine.CharacterMovementComponent|SetMaxWalkSpeed (Variables|Character|GetCharacterMovement) (Variables|Default|GetMaxWalkingSpeed)))

(fn Rotate
  (params (Scale :type Float%20%28double-precision%29))
  (Pawn|Input|AddControllerYawInput (* Scale (Utilities|Time|GetWorldDeltaSeconds) 0.0)))

(fn DrainStamina
  (params (B :type Float%20%28double-precision%29))
  (bind _output_get (Variables|Default|SetCurrentStamina (Math|Float|Clamp(Float) (- (Variables|Default|GetCurrentStamina) (* (Variables|Default|GetStaminaDrainRate) B)) 0.0 (Variables|Default|GetMaxStamina))))
  (return _output_get))

(fn RegenerateStamina
  (params (A :type Float%20%28double-precision%29))
  (Variables|Default|SetCurrentStamina (Math|Float|Clamp(Float) (+ (Variables|Default|GetCurrentStamina) (* A (Variables|Default|GetStaminaRegenRate))) 0.0 (Variables|Default|GetMaxStamina))))

(fn ComputeBodyPartsLocation
  (Utilities|FlowControl|Sequence
    (:then_0
      (Utilities|Map|Add (Variables|Default|GetBodyPartsLocation) "Head" (Transformation|GetSocketLocation (Variables|Character|GetMesh) "HeadSocket"))
      (Utilities|Map|Add (Variables|Default|GetBodyPartsLocation) "Body" (Transformation|GetSocketLocation (Variables|Character|GetMesh) "BodySocket"))
      (Utilities|Map|Add (Variables|Default|GetBodyPartsLocation) "RightLeg" (Transformation|GetSocketLocation (Variables|Character|GetMesh) "RightLegSocket")))
    (:then_1
      (Utilities|Map|Add (Variables|Default|GetBodyPartsLocation) "LeftLeg" (Transformation|GetSocketLocation (Variables|Character|GetMesh) "LeftLegSocket"))
      (Utilities|Map|Add (Variables|Default|GetBodyPartsLocation) "LeftArm" (Transformation|GetSocketLocation (Variables|Character|GetMesh) "LeftArmSocket"))
      (Utilities|Map|Add (Variables|Default|GetBodyPartsLocation) "RightArm" (Transformation|GetSocketLocation (Variables|Character|GetMesh) "RightArmSocket")))))

(fn TrySetCurrentRockRef
  (params (HitActor :type Actor%20Object%20Reference))
  (if (Utilities|IsValid (Variables|Default|GetCurrentRockRef))
    (Rendering|SetVisibility (Variables|/Game/Inventory/BP_PickUpStone.BP_PickUpStone_C|GetInteract (Variables|Default|GetCurrentRockRef)) false false))
  (bind _asbp_pick_up_stone (Utilities|Casting|CastToBP_PickUpStone HitActor)
    (:then
      (if (Utilities|IsValid (Variables|Default|GetCurrentKnifeRef))
        (Rendering|SetVisibility (Variables|/Game/Inventory/BP_Projectile.BP_Projectile_C|GetInteract (Variables|Default|GetCurrentKnifeRef)) false false))
      (Variables|Default|SetCurrentKnifeRef 0)
      (bind _output_get (Variables|Default|SetCurrentRockRef _asbp_pick_up_stone))
      (Rendering|SetVisibility (Variables|/Game/Inventory/BP_PickUpStone.BP_PickUpStone_C|GetInteract _output_get) true false))
    (:CastFailed
      (CallFunction|TrySetCurrentKnifeRef HitActor)
      (if (Utilities|IsValid (Variables|Default|GetCurrentRockRef))
        (Rendering|SetVisibility (Variables|/Game/Inventory/BP_PickUpStone.BP_PickUpStone_C|GetInteract (Variables|Default|GetCurrentRockRef)) false false))
      (Variables|Default|SetCurrentRockRef 0))))

(fn TrySetCurrentKnifeRef
  (params (Actor :type Actor%20Object%20Reference))
  (bind _asbp_projectile (Utilities|Casting|CastToBP_Projectile Actor)
    (:then
      (Variables|Default|SetCurrentRockRef 0)
      (bind _output_get (Variables|Default|SetCurrentKnifeRef _asbp_projectile))
      (Rendering|SetVisibility (Variables|/Game/Inventory/BP_Projectile.BP_Projectile_C|GetInteract _output_get) true false))
    (:CastFailed
      (if (Utilities|IsValid (Variables|Default|GetCurrentKnifeRef))
        (Rendering|SetVisibility (Variables|/Game/Inventory/BP_Projectile.BP_Projectile_C|GetInteract (Variables|Default|GetCurrentKnifeRef)) false false)
        (Variables|Default|SetCurrentKnifeRef 0)))))

(fn IsWalking
  (bind _asbp_player_pawn (Utilities|Casting|CastToBP_PlayerPawn (Game|Player|GetPlayerPawn 0)))
  (return (and (Pawn|Components|CharacterMovement|IsWalking (Variables|/Script/Engine.Character|GetCharacterMovement _asbp_player_pawn)) (not (< (Math|Vector|VectorLength (Transformation|GetVelocity)) 1.0)))))

(fn CheckStaminaLevel
  (params (Stamina :type Float%20%28double-precision%29))
  (if (<= Stamina 0.0)
    (Variables|Default|SetIsSprinting false)
    (bind _asbp_player_pawn (Utilities|Casting|CastToBP_PlayerPawn (Game|Player|GetPlayerPawn 0)))
    (Variables|/Script/Engine.CharacterMovementComponent|SetMaxWalkSpeed (Variables|/Script/Engine.Character|GetCharacterMovement _asbp_player_pawn) (Variables|Default|GetMaxWalkingSpeed))))

(fn CalculatePickUpRange
  (bind _camera (Variables|Default|GetCamera))
  (bind _returnvalue (Transformation|GetWorldLocation _camera))
  (return _returnvalue (+ _returnvalue (* (Math|Vector|GetForwardVector _camera) (Variables|Default|GetPickUpDistance)))))

(fn IsFalling
  (return (AI|Components|NavMovement|IsFalling (Variables|Character|GetCharacterMovement))))

(fn GetStamina
  (return (Variables|Default|GetCurrentStamina)))

(fn HasStaminaforJump
  (return (and (>= (CallFunction|GetStamina) 1e+01) (not (CallFunction|IsFalling)))))

(fn StaminaJump
  (Variables|Default|SetCurrentStamina (- (Variables|Default|GetCurrentStamina) 1e+01)))

(fn TryUpdateNumOfRocks
  (bind _currentrockref (Variables|Default|GetCurrentRockRef))
  (if (Utilities|IsValid _currentrockref)
    (bind _foundwidgets (Widget|GetAllWidgetsOfClass "/Game/HUDComponents/WB_HUD.WB_HUD_C" true))
    (Default|UpdateNumbers (Variables|/Game/HUDComponents/WB_HUD.WB_HUD_C|GetHotbarWidget (Utilities|Array|Get(acopy) _foundwidgets)) (Variables|/Game/Inventory/BP_PickUpStone.BP_PickUpStone_C|GetItemId _currentrockref))
    (Actor|DestroyActor (Variables|Default|GetCurrentRockRef))))

(fn TryUpdateNumOfKnives
  (bind _currentkniferef (Variables|Default|GetCurrentKnifeRef))
  (if (Utilities|IsValid _currentkniferef)
    (bind _foundwidgets (Widget|GetAllWidgetsOfClass "/Game/HUDComponents/WB_HUD.WB_HUD_C" true))
    (Default|UpdateNumbers (Variables|/Game/HUDComponents/WB_HUD.WB_HUD_C|GetHotbarWidget (Utilities|Array|Get(acopy) _foundwidgets)) (Variables|/Game/Inventory/BP_Projectile.BP_Projectile_C|GetItemId _currentkniferef))
    (Actor|DestroyActor (Variables|Default|GetCurrentKnifeRef))))

(fn TakeDamage
  (params (Damage :type Float%20%28double-precision%29))
  (Variables|Default|SetHealth (Math|Float|Clamp(Float) (- (Variables|Default|GetHealth) Damage) 0.0 1e+02)))

(fn MakeSound
  (bind _returnvalue (Transformation|GetVelocity))
  (if (== (.z _returnvalue) 0.0)
    (Class|PawnNoiseEmitterComponent|MakeNoise (Variables|Default|GetPawnNoiseEmitter) self (/ (Math|Vector|VectorLength (Math|Vector|MakeVector (.x _returnvalue) (.y _returnvalue) 0.0)) (Variables|Default|GetMaxWalkingSpeed)) (Transformation|GetActorLocation))))

(fn HandleStamina
  (params (DeltaSeconds :type Float%20%28double-precision%29))
  (if (Variables|Default|GetIsSprinting)
    (bind _iswalking (CallFunction|IsWalking))
    (if _iswalking
      (bind _output_get (CallFunction|DrainStamina DeltaSeconds))
      (CallFunction|CheckStaminaLevel _output_get)
      (else
        (CallFunction|RegenerateStamina DeltaSeconds :!label _label)))
    (else
      (goto _label))))

(fn IsAlive
  (return (> (Variables|Default|GetHealth) 0.0)))

(fn StopGame
  (params (Alive :type Boolean))
  (if (not Alive)
    (Game|OpenLevel(byObjectReference) "/Game/DeathScreen/DeathScreenLevel.DeathScreenLevel")))

(fn QuestIsCompleted
  (params (QuestID :type Integer))
  (return (.IsCompleted (Utilities|Struct|BreakQuestStructure (Utilities|Array|Get(acopy) (Variables|Default|GetQuestsArray) QuestID)))))

(fn WinGame
  (Game|OpenLevel(byObjectReference) "/Game/GameWon.GameWon"))

(fn CompleteQuest
  (params (QuestID :type Integer))
  (bind _questsarray (Variables|Default|GetQuestsArray))
  (bind _output (Utilities|Array|Get(acopy) _questsarray QuestID))
  (bind (_questid _title _objectivetext) (Utilities|Struct|BreakQuestStructure _output))
  (Utilities|Array|SetArrayElem _questsarray QuestID (Utilities|Struct|MakeQuestStructure _questid _title _objectivetext true)))