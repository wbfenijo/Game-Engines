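; BP_PickUpStone is a stone actor that shows an interact component and creates a noise source when it hits something.
; On Tick, while the player pawn is nearby, it rotates the Interact component to face the player camera.
; On Hit, it spawns a ThrowableNoiseEmitterPawn at the impact location, with no filtering or limit on repeated hits.
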(event EventBeginPlay)

(event Collision|EventActorBeginOverlap
  (params (OtherActor :type Actor%20Object%20Reference)))

(event EventTick
  (params (DeltaSeconds :type Float%20%28single-precision%29))
  (bind _interact (Variables|Default|GetInteract))
  (if (< (Transformation|GetDistanceTo (Game|Player|GetPlayerPawn 0)) 3e+02)
    (Transformation|SetWorldRotation _interact (Math|Rotator|FindLookatRotation (Transformation|GetWorldLocation _interact) (Camera|GetCameraLocation (Game|GetPlayerCameraManager 0))) false false)))

(event Collision|EventHit
  (params (MyComp :type Primitive%20Component%20Object%20Reference) (Other :type Actor%20Object%20Reference) (OtherComp :type Primitive%20Component%20Object%20Reference) (bSelfMoved :type Boolean) (HitLocation :type Vector :default "0, 0, 0") (HitNormal :type Vector :default "0, 0, 0") (NormalImpulse :type Vector :default "0, 0, 0") (Hit :type Hit%20Result%20Structure%20%28by%20ref%29))
  (Game|SpawnActorfromClass "/Game/Inventory/ThrowableNoiseEmitterPawn.ThrowableNoiseEmitterPawn_C" (Math|Transform|MakeTransform HitLocation "0, 0, 0" "1.000000,1.000000,1.000000") "Undefined" "MultiplyWithRoot" 0 0))

(fn ConstructionScript)